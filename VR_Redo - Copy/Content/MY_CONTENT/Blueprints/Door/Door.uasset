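; Interactive door with a mail flap that stays locked until a letter exchange completes.
; The first knock opens the flap and spawns a Letter; after it leaves the box, a delayed Tick check snaps a released, returned letter into place and triggers its end animation.
; An externally set CloseBox flag closes the flap and unlocks the door, letting an MC-tagged component on the handle swing it open via MoveComponentTo.
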(event OnComponentBeginOverlap(KnockBox)
  (params (OverlappedComponent :type Primitive%20Component%20Object%20Reference) (OtherActor :type Actor%20Object%20Reference) (OtherComp :type Primitive%20Component%20Object%20Reference) (OtherBodyIndex :type Integer) (bFromSweep :type Boolean) (SweepResult :type Hit%20Result%20Structure%20%28by%20ref%29))
  (if (not (== (Utilities|GetClass OtherActor) "/Game/MY_CONTENT/Blueprints/Door/Letter.Letter_C"))
    (Audio|PlaySoundatLocation "/Game/MY_CONTENT/Audio/knockTrimmed.knockTrimmed" (Transformation|GetWorldLocation (Variables|Default|GetKnockBox)) "0, 0, 0" 1.0 1.0 0.0 0 0 0)
    (if (not (Variables|Default|GetSpawnedLetter))
      (Variables|Default|SetSpawnedLetter true)
      (Utilities|FlowControl|Delay 1.0)
      (Utilities|OpenFlap))))

(event OnComponentBeginOverlap(Handle)
  (params (OverlappedComponent :type Primitive%20Component%20Object%20Reference) (OtherActor :type Actor%20Object%20Reference) (OtherComp :type Primitive%20Component%20Object%20Reference) (OtherBodyIndex :type Integer) (bFromSweep :type Boolean) (SweepResult :type Hit%20Result%20Structure%20%28by%20ref%29))
  (if (and (Components|ComponentHasTag OtherComp "MC") (Variables|Default|GetUnlocked))
    (Utilities|OpenDoor)
    (else
      (Development|PrintString (Utilities|String|Append " 
 
 
 
 
 
 
 
 
 
 
                               " "Locked")))))

(event OnComponentEndOverlap(Box)
  (params (OverlappedComponent :type Primitive%20Component%20Object%20Reference) (OtherActor :type Actor%20Object%20Reference) (OtherComp :type Primitive%20Component%20Object%20Reference) (OtherBodyIndex :type Integer))
  (if (== (Utilities|GetClass OtherActor) "/Game/MY_CONTENT/Blueprints/Door/Letter.Letter_C")
    (Variables|Default|SetLetterSubmitDelay true)))

(event Custom|EndSubmitDelay
  ;[1 1 1] Delay Timer
  (Variables|Default|SetStartSubmitCheck true))

(event EventBeginPlay)

(event Collision|EventActorBeginOverlap
  (params (OtherActor :type Actor%20Object%20Reference)))

(event EventTick
  (params (DeltaSeconds :type Float%20%28single-precision%29))
  (bind _box (Variables|Default|GetBox))
  (bind _overlappingactors (Collision|GetOverlappingActors _box "/Game/MY_CONTENT/Blueprints/Door/Letter.Letter_C" :!class /Script/Engine.PrimitiveComponent))
  (Utilities|FlowControl|Sequence
    (:then_0
      (if (Variables|Default|GetCloseBox)
        (Variables|Default|SetCloseBox false)
        (Variables|Default|SetUnlocked true)
        (Utilities|CloseFlap)))
    (:then_1
      ;[1 1 1] Delay Timer
      (if (Variables|Default|GetLetterSubmitDelay)
        (Utilities|Time|SetTimerbyEvent (delegate Custom|EndSubmitDelay) 2.0)
        (Variables|Default|SetLetterSubmitDelay false)
        (else
          ;[1 1 1] Submit letter check
          (if (and (> (Utilities|Array|Length _overlappingactors) 0) (Variables|Default|GetStartSubmitCheck))
            (if (and (not (Variables|Default|GetSubmittedLetter)) (not (Variables|/Game/VRTemplate/Blueprints/GrabComponent.GrabComponent_C|GetbIsHeld (Actor|GetComponentbyClass (Utilities|Array|Get(acopy) _overlappingactors) "/Game/VRTemplate/Blueprints/GrabComponent.GrabComponent_C"))))
              (Variables|Default|SetSubmittedLetter true)
              ;[1 1 1] Submit letter
              (bind _returnvalue (Actor|GetActorOfClass "/Game/MY_CONTENT/Blueprints/Door/Letter.Letter_C"))
              (Transformation|SetActorLocationAndRotation _returnvalue (Transformation|GetWorldLocation (Variables|Default|GetLetterBoxBase)) (Math|Rotator|MakeRotator 0.0 0.0 (+ (.yaw (Transformation|GetActorRotation self)) 1.8e+02)))
              (Components|DestroyComponent (Variables|/Game/MY_CONTENT/Blueprints/Door/Letter.Letter_C|GetGrabComponent _returnvalue))
              (Variables|/Game/MY_CONTENT/Blueprints/Door/Letter.Letter_C|SetEndAnim _returnvalue true))))))))

(fn ConstructionScript)