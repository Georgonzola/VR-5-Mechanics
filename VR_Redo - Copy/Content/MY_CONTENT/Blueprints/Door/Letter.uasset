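; Letter actor that animates between its spawn point and the Door's letterbox, then removes itself.
; On BeginPlay it caches the path to LetterBoxBase, and Tick linearly moves it there over half a second using a timer.
; It then reverses the path and waits for EndAnim, which is not set true in this graph.
; The return trip ends by setting CloseBox on the Door and destroying the letter.
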(event EventBeginPlay
  (Variables|Default|SetStartLocation (Transformation|GetActorLocation))
  (bind _returnvalue (Actor|GetActorOfClass "/Game/MY_CONTENT/Blueprints/Door/Door.Door_C"))
  (Variables|Default|SetEndLocation (Transformation|GetWorldLocation (Variables|/Game/MY_CONTENT/Blueprints/Door/Door.Door_C|GetLetterBoxBase _returnvalue)))
  (Variables|Default|SetDistance (- (Variables|Default|GetEndLocation) (Variables|Default|GetStartLocation))))

(event EventTick
  (params (DeltaSeconds :type Float%20%28single-precision%29))
  (if (Variables|Default|GetInitAnim)
    (if (Variables|Default|GetEndAnim)
      (bind _output_get (Variables|Default|SetTimer (+ (stale _output_get) (Utilities|Time|GetWorldDeltaSeconds))))
      (if (>= (Variables|Default|GetTimer) 0.5)
        (Variables|Default|SetEndAnim false)
        (bind _returnvalue (Actor|GetActorOfClass "/Game/MY_CONTENT/Blueprints/Door/Door.Door_C"))
        (Variables|/Game/MY_CONTENT/Blueprints/Door/Door.Door_C|SetCloseBox _returnvalue true)
        (Actor|DestroyActor)
        (else
          (Transformation|SetActorLocation (+ (Variables|Default|GetStartLocation) (* (Variables|Default|GetDistance) (* (Variables|Default|GetTimer) 2.0))) false false))))
    (else
      (bind _output_get_2 (Variables|Default|SetTimer (+ (stale _output_get_2) (Utilities|Time|GetWorldDeltaSeconds))))
      (if (>= (Variables|Default|GetTimer) 0.5)
        (Variables|Default|SetInitAnim true)
        (Variables|Default|SetTimer 0.0)
        (Variables|Default|SetEndLocation (Variables|Default|GetStartLocation))
        (bind _returnvalue_2 (Actor|GetActorOfClass "/Game/MY_CONTENT/Blueprints/Door/Door.Door_C"))
        (Variables|Default|SetStartLocation (Transformation|GetWorldLocation (Variables|/Game/MY_CONTENT/Blueprints/Door/Door.Door_C|GetLetterBoxBase _returnvalue_2)))
        (Variables|Default|SetDistance (- (Variables|Default|GetEndLocation) (Variables|Default|GetStartLocation)))
        (else
          (Transformation|SetActorLocation (+ (Variables|Default|GetStartLocation) (* (Variables|Default|GetDistance) (* (Variables|Default|GetTimer) 2.0))) false false))))))

(fn ConstructionScript)