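; Pressable button actor that triggers when something overlaps its Box, used for menu hand switching or a fanfare.
; An IsActive flag blocks retriggers, and the actor's menuLeft or menuRight tag calls SwitchHand on the HandSwitcher with true or false.
; Without either tag it plays the Fanfare sound.
; The Animation graph then eases the Button component in and back along local Y before clearing the flag.
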(event OnComponentBeginOverlap(Box)
  (params (OverlappedComponent :type Primitive%20Component%20Object%20Reference) (OtherActor :type Actor%20Object%20Reference) (OtherComp :type Primitive%20Component%20Object%20Reference) (OtherBodyIndex :type Integer) (bFromSweep :type Boolean) (SweepResult :type Hit%20Result%20Structure%20%28by%20ref%29))
  (if (not (Variables|Default|GetIsActive))
    (Variables|Default|SetIsActive true)
    (Utilities|FlowControl|Sequence
      (:then_0
        (if (Actor|ActorHasTag "menuLeft")
          (bind _returnvalue (Actor|GetActorOfClass "/Game/MY_CONTENT/Blueprints/Menu/HandSwitcher.HandSwitcher_C"))
          (Default|SwitchHand _returnvalue true)
          (elif (Actor|ActorHasTag "menuRight")
            (bind _returnvalue_2 (Actor|GetActorOfClass "/Game/MY_CONTENT/Blueprints/Menu/HandSwitcher.HandSwitcher_C"))
            (Default|SwitchHand _returnvalue_2 false)
            (else
              (Audio|PlaySound2D "/Game/MY_CONTENT/Audio/fanfare.fanfare" 1.0 1.0 0.0 0 0)))))
      (:then_1
        (Utilities|Animation)))))

(event EventBeginPlay)

(event Collision|EventActorBeginOverlap
  (params (OtherActor :type Actor%20Object%20Reference)))

(event EventTick
  (params (DeltaSeconds :type Float%20%28single-precision%29)))

(fn ConstructionScript)