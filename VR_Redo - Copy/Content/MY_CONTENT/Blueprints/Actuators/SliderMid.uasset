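; VR slider actuator that a held motion controller drags to set the Car's height or volume, chosen by actor tag.
; While held, the controller's world Z or X, picked from the actor's pitch at BeginPlay, maps to a clamped, scale-aware slider offset.
; Holding B or X snaps the value to 25-unit notches.
; If the controller leaves the Box, VRPawn detaches it.
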(event EventBeginPlay
  ;[1 1 1] Set Vertical
  (Variables|Default|SetVertical (< (.pitch (Transformation|GetActorRotation)) 45.0))
  (Variables|Default|SetOffset (* (.x (Transformation|GetActorScale3D)) 2.7e+02)))

(event Collision|EventActorBeginOverlap
  (params (OtherActor :type Actor%20Object%20Reference)))

(event EventTick
  (params (DeltaSeconds :type Float%20%28single-precision%29))
  (bind _offset (Variables|Default|GetOffset))
  (bind _grabcomponent (Variables|Default|GetGrabComponent))
  (bind _sliderbase (Variables|Default|GetSliderBase))
  (bind _sliderbase_2 (Variables|Default|GetSliderBase))
  (bind _offset_2 (Variables|Default|GetOffset))
  (bind _grabcomponent_2 (Variables|Default|GetGrabComponent))
  (bind _returnvalue (Transformation|GetWorldTransform _sliderbase))
  (bind _returnvalue_2 (Transformation|GetWorldTransform _sliderbase_2))
  (bind _motioncontrollerref (Variables|/Game/VRTemplate/Blueprints/GrabComponent.GrabComponent_C|GetMotionControllerRef _grabcomponent))
  (bind _motioncontrollerref_2 (Variables|/Game/VRTemplate/Blueprints/GrabComponent.GrabComponent_C|GetMotionControllerRef _grabcomponent_2))
  (if (Variables|/Game/VRTemplate/Blueprints/GrabComponent.GrabComponent_C|GetbIsHeld (Variables|Default|GetGrabComponent))
    ;[1 1 1] Checks whether controller is in reasonable range
    (Variables|Default|SetOverlap false)
    (for _array_element (Class|PrimitiveComponent|GetOverlappingComponents (Variables|Default|GetBox))
      (if (== _array_element (Components|GetChildComponent (Variables|/Game/VRTemplate/Blueprints/GrabComponent.GrabComponent_C|GetMotionControllerRef (Variables|Default|GetGrabComponent)) 0))
        (bind _output_get (Variables|Default|SetOverlap true))))
    (if _output_get
      (Utilities|FlowControl|Sequence
        (:then_0
          (if (Variables|Default|GetVertical)
            (bind _motioncontrollerdata (Class|HeadMountedDisplayFunctionLibrary|GetMotionControllerData _motioncontrollerref (Utilities|GetHand _motioncontrollerref)))
            (Variables|Default|SetSliderValue (Math|Float|MapRangeClamped (.z (.aimposition _motioncontrollerdata)) (+ (.z (.location _returnvalue_2)) _offset) (- (.z (.location _returnvalue_2)) _offset) -2.5e+02 2.5e+02))
            (else
              (bind _motioncontrollerdata_2 (Class|HeadMountedDisplayFunctionLibrary|GetMotionControllerData _motioncontrollerref_2 (Utilities|GetHand _motioncontrollerref_2)))
              (Variables|Default|SetSliderValue (Math|Float|MapRangeClamped (.x (.aimposition _motioncontrollerdata_2)) (+ (.x (.location _returnvalue)) _offset_2) (- (.x (.location _returnvalue)) _offset_2) -2.5e+02 2.5e+02)))))
        (:then_1
          ;[1 1 1] Round value to nearest 5
          (if (Variables|Default|GetDoNotch)
            (if (>= (Math|Float|%(Float) (Variables|Default|GetSliderValue) 25.0) 12.5)
              (Variables|Default|SetSliderValue (+ (Variables|Default|GetSliderValue) (- 25.0 (Math|Float|%(Float) (Variables|Default|GetSliderValue) 25.0))))
              (else
                (Variables|Default|SetSliderValue (- (Variables|Default|GetSliderValue) (Math|Float|%(Float) (Variables|Default|GetSliderValue) 25.0)))))))
        (:then_2
          ;[1 1 1] Set Slider Location
          (Transformation|SetRelativeLocation (Variables|Default|GetSlider) (Math|Vector|MakeVector 0.0 (Variables|Default|GetSliderValue) 0.0) false false))
        (:then_3
          (Utilities|FlowControl|Sequence
            (:then_0
              (if (Actor|ActorHasTag "carSliderHeight")
                (bind _returnvalue_3 (Actor|GetActorOfClass "/Game/MY_CONTENT/Blueprints/Menu/Car.Car_C"))
                (Default|SetHeight _returnvalue_3 (Variables|Default|GetSliderValue))))
            (:then_1
              (if (Actor|ActorHasTag "carSliderVolume")
                (bind _returnvalue_4 (Actor|GetActorOfClass "/Game/MY_CONTENT/Blueprints/Menu/Car.Car_C"))
                (Default|SetVolume _returnvalue_4 (Variables|Default|GetSliderValue)))))))
      (else
        ;[1 1 1] Detach controller If out of range
        (bind _returnvalue_5 (Actor|GetActorOfClass "/Game/VRTemplate/Blueprints/VRPawn.VRPawn_C"))
        (Default|ActuatorDetach _returnvalue_5 (Utilities|Enum|Equal(Enum) (Utilities|GetHand (Variables|/Game/VRTemplate/Blueprints/GrabComponent.GrabComponent_C|GetMotionControllerRef (Variables|Default|GetGrabComponent))) "Left"))))
    (else
      (Variables|Default|SetDoNotch false))))

(event EventARelease
  ;[1 1 1] Whether to set slider value to notches of 5
  (Variables|Default|SetDoNotch false))

(event EventButtonB
  ;[1 1 1] Whether to set slider value to notches of 5
  (Variables|Default|SetDoNotch true))

(event EventButtonX
  ;[1 1 1] Whether to set slider value to notches of 5
  (Variables|Default|SetDoNotch true))

(event EventXRelease
  ;[1 1 1] Whether to set slider value to notches of 5
  (Variables|Default|SetDoNotch false))

(fn ConstructionScript)