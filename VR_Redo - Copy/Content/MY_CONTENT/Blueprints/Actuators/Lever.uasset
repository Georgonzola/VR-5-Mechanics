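; VR lever actuator that the player grabs with a motion controller to switch an IsOn state.
; While held, Tick maps the controller aim position's local Z to a clamped lever roll, so it follows the hand in the actor's own space.
; IsOn flips only at either end of travel.
; If the controller stops overlapping the Sphere, VRPawn detaches it; an older world-axis mapping remains unconnected.
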(event EventTick
  (params (DeltaSeconds :type Float%20%28single-precision%29))
  (bind _grabcomponent (Variables|Default|GetGrabComponent))
  (bind _motioncontrollerref (Variables|/Game/VRTemplate/Blueprints/GrabComponent.GrabComponent_C|GetMotionControllerRef _grabcomponent))
  (if (Variables|/Game/VRTemplate/Blueprints/GrabComponent.GrabComponent_C|GetbIsHeld (Variables|Default|GetGrabComponent))
    ;[1 1 1] Checks whether controller is in reasonable range
    (Variables|Default|SetOverlap false)
    (for _array_element (Class|PrimitiveComponent|GetOverlappingComponents (Variables|Default|GetSphere))
      (if (== _array_element (Components|GetChildComponent (Variables|/Game/VRTemplate/Blueprints/GrabComponent.GrabComponent_C|GetMotionControllerRef (Variables|Default|GetGrabComponent)) 0))
        (bind _output_get (Variables|Default|SetOverlap true))))
    (if _output_get
      (Utilities|FlowControl|Sequence
        (:then_0
          (bind _motioncontrollerdata (Class|HeadMountedDisplayFunctionLibrary|GetMotionControllerData _motioncontrollerref (Utilities|GetHand _motioncontrollerref)))
          (Variables|Default|SetLeverValue (Math|Float|MapRangeClamped (.z (.location (Math|Transform|MakeRelativeTransform (Math|Transform|MakeTransform (.aimposition _motioncontrollerdata) (Class|KismetMathLibrary|QuatRotator (.aimrotation _motioncontrollerdata))) (Transformation|GetActorTransform self)))) 3.2 -3.2 68.0 -68.0)))
        (:then_1
          ;[1 1 1] Set Lever rotation
          (Transformation|SetRelativeRotation (Variables|Default|GetLever) (Math|Rotator|MakeRotator (Variables|Default|GetLeverValue) 0.0 0.0) false false))
        (:then_2
          ;[1 1 1] Set IsOn status
          (Utilities|FlowControl|Sequence
            (:then_0
              (if (and (Variables|Default|GetIsOn) (>= (Variables|Default|GetLeverValue) 68.0))
                (Variables|Default|SetIsOn false)))
            (:then_1
              (if (and (not (Variables|Default|GetIsOn)) (<= (Variables|Default|GetLeverValue) -68.0))
                (Variables|Default|SetIsOn true))))))
      (else
        ;[1 1 1] Detach controller If out of range
        (bind _returnvalue (Actor|GetActorOfClass "/Game/VRTemplate/Blueprints/VRPawn.VRPawn_C"))
        (Default|ActuatorDetach _returnvalue (Utilities|Enum|Equal(Enum) (Utilities|GetHand (Variables|/Game/VRTemplate/Blueprints/GrabComponent.GrabComponent_C|GetMotionControllerRef (Variables|Default|GetGrabComponent))) "Left"))
        (Development|PrintString (Utilities|String|Append " 
 
 
 
 
 
 
 
 
 
 
 
 
                                    " "FAR"))))))

(fn ConstructionScript)