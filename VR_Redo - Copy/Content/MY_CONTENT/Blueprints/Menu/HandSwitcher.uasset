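; HandSwitcher is a menu actor that toggles a setting between left and right hand.
; SwitchHand stores the choice in IsLeft and highlights the chosen text label in white, turning the other black.
; It then sets both active inventory items on the VRPawn to the same fixed index.
; Finally it finds both radial menu actors by class and passes IsLeft to their widgets' SwitchIcons.
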(event EventBeginPlay)

(event Collision|EventActorBeginOverlap
  (params (OtherActor :type Actor%20Object%20Reference)))

(event EventTick
  (params (DeltaSeconds :type Float%20%28single-precision%29)))

(fn ConstructionScript)

(fn SwitchHand
  (params (Left :type Boolean))
  (if Left
    (Rendering|Components|TextRender|SetTextRenderColor (Variables|Default|GetLeft) (Variables|Default|GetWhite))
    (Rendering|Components|TextRender|SetTextRenderColor (Variables|Default|GetRight) (Variables|Default|GetBlack))
    (Variables|Default|SetIsLeft true)
    (else
      (Rendering|Components|TextRender|SetTextRenderColor (Variables|Default|GetRight) (Variables|Default|GetWhite))
      (Rendering|Components|TextRender|SetTextRenderColor (Variables|Default|GetLeft) (Variables|Default|GetBlack))
      (Variables|Default|SetIsLeft false)))
  (bind _returnvalue (Actor|GetActorOfClass "/Game/VRTemplate/Blueprints/VRPawn.VRPawn_C"))
  (Default|SetActiveInventoryItemLeft _returnvalue 1)
  (Default|SetActiveInventoryItemRight _returnvalue 1)
  (Utilities|FlowControl|Sequence
    (:then_0
      (bind _returnvalue_2 (Actor|GetActorOfClass "/Game/MY_CONTENT/Blueprints/Inventory/RadialMenuLeft.RadialMenuLeft_C"))
      (bind _asradial_menu_left_w (Utilities|Casting|CastToRadialMenuLeft_W (UserInterface|GetUserWidgetObject (Variables|/Game/MY_CONTENT/Blueprints/Inventory/RadialMenuLeft.RadialMenuLeft_C|GetWidget _returnvalue_2))))
      (Default|SwitchIcons _asradial_menu_left_w (Variables|Default|GetIsLeft)))
    (:then_1
      (bind _returnvalue_3 (Actor|GetActorOfClass "/Game/MY_CONTENT/Blueprints/Inventory/RadialMenuRight.RadialMenuRight_C"))
      (bind _asradial_menu_right_w (Utilities|Casting|CastToRadialMenuRight_W (UserInterface|GetUserWidgetObject (Variables|/Game/MY_CONTENT/Blueprints/Inventory/RadialMenuRight.RadialMenuRight_C|GetWidget _returnvalue_3))))
      (Default|SwitchIcons _asradial_menu_right_w (Variables|Default|GetIsLeft)))))