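; Menu car actor that honks when a component tagged MC overlaps its box and formats slider-style values for volume and height.
; The overlap plays the horn at the steering wheel and prints a debug message.
; SetVolume remaps its input to a percentage label and a Master sound class override through MasterMix.
; SetHeight only updates a feet-and-inches label; the horn sound created at BeginPlay is unused here.
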(event OnComponentBeginOverlap(Box)
  (params (OverlappedComponent :type Primitive%20Component%20Object%20Reference) (OtherActor :type Actor%20Object%20Reference) (OtherComp :type Primitive%20Component%20Object%20Reference) (OtherBodyIndex :type Integer) (bFromSweep :type Boolean) (SweepResult :type Hit%20Result%20Structure%20%28by%20ref%29))
  (if (Components|ComponentHasTag OtherComp "MC")
    (Development|PrintString (Utilities|String|Append " 
 
 
 
 
 
 
 
 
 
 
 
 
                          " "HIT"))
    (Audio|PlaySoundatLocation "/Game/MY_CONTENT/Audio/carhorn.carhorn" (Transformation|GetWorldLocation (Variables|Default|GetSteering%20wheel)) "0, 0, 0" 1.0 1.0 0.0 0 0 0)))

(event EventBeginPlay
  (bind _returnvalue (Audio|CreateSound2D "/Game/MY_CONTENT/Audio/carhorn.carhorn" 1.0 1.0 0.0 0))
  (Variables|Default|SetHorn _returnvalue))

(event Collision|EventActorBeginOverlap
  (params (OtherActor :type Actor%20Object%20Reference)))

(event EventTick
  (params (DeltaSeconds :type Float%20%28single-precision%29)))

(fn ConstructionScript)

(fn SetVolume
  (params (Value :type Float%20%28single-precision%29))
  (bind _returnvalue (Math|Float|MapRangeClamped Value -2.5e+02 2.5e+02 0.0 1e+02))
  (Rendering|Components|TextRender|SetText (Variables|Default|GetVolumeText) (Utilities|Text|ToText(String) (Utilities|String|Append "Volume: " (Utilities|String|ToString(Integer) (Math|Float|Floor _returnvalue)))))
  (Audio|SetSoundMixClassOverride "/Game/MY_CONTENT/Audio/MasterMix.MasterMix" "/Engine/EngineSounds/Master.Master" (/ _returnvalue 5e+01) 1.0 0.0 true)
  (Audio|PushSoundMixModifier "/Game/MY_CONTENT/Audio/MasterMix.MasterMix"))

(fn SetHeight
  (params (Value :type Float%20%28single-precision%29))
  (bind _returnvalue (Math|Float|MapRangeClamped Value -2.5e+02 2.5e+02 54.0 78.0))
  (Rendering|Components|TextRender|SetText (Variables|Default|GetHeightText) (Utilities|Text|ToText(String) (Utilities|String|Append "Height: " (Utilities|String|ToString(Integer) (Math|Float|Floor (/ _returnvalue 12.0))) "'" (Utilities|String|ToString(Integer) (Math|Float|Floor (Math|Float|%(Float) _returnvalue 12.0)))))))