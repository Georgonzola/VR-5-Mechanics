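; VR inventory key fob with a flip-out key that triggers the pawn's teleport.
; B/Y presses Button2, then swings the key open, or if already open calls KeyTeleport on the VRPawn and closes it.
; A/X presses Button1, then closes the key if open.
; The PushAnim macro eases the chosen button in and back out, and MoveComponentTo rotates the key between open and closed.
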(event EventBeginPlay)

(event Collision|EventActorBeginOverlap
  (params (OtherActor :type Actor%20Object%20Reference)))

(event EventTick
  (params (DeltaSeconds :type Float%20%28single-precision%29)))

(event EventButtonA
  (bind _key (Variables|Default|GetKey))
  (Utilities|PushAnim true
    (:end
      (if (Variables|Default|GetKeyOpen)
        (Variables|Default|SetKeyOpen false)
        (Components|MoveComponentTo _key (.location (Transformation|GetRelativeTransform _key)) (Variables|Default|GetClosedRotator) false false 0.2 true)))))

(event EventButtonB
  (bind _key (Variables|Default|GetKey))
  (bind _key_2 (Variables|Default|GetKey))
  (Utilities|PushAnim false
    (:end
      (if (Variables|Default|GetKeyOpen)
        (Development|PrintString (Utilities|String|Append "  
 
 
 
 
 
 
 
 
 
 
 
 
                                     " "Teleport"))
        (bind _returnvalue (Actor|GetActorOfClass "/Game/VRTemplate/Blueprints/VRPawn.VRPawn_C"))
        (Default|KeyTeleport _returnvalue)
        (if (Variables|Default|GetKeyOpen)
          (Variables|Default|SetKeyOpen false)
          (Components|MoveComponentTo _key_2 (.location (Transformation|GetRelativeTransform _key_2)) (Variables|Default|GetClosedRotator) false false 0.2 true))
        (else
          (Variables|Default|SetKeyOpen true)
          (Components|MoveComponentTo _key (.location (Transformation|GetRelativeTransform _key)) (Variables|Default|GetOpenRotator) false false 0.2 true))))))

(event EventButtonX
  (bind _key (Variables|Default|GetKey))
  (Utilities|PushAnim true
    (:end
      (if (Variables|Default|GetKeyOpen)
        (Variables|Default|SetKeyOpen false)
        (Components|MoveComponentTo _key (.location (Transformation|GetRelativeTransform _key)) (Variables|Default|GetClosedRotator) false false 0.2 true)))))

(event EventButtonY
  (bind _key (Variables|Default|GetKey))
  (bind _key_2 (Variables|Default|GetKey))
  (Utilities|PushAnim false
    (:end
      (if (Variables|Default|GetKeyOpen)
        (Development|PrintString (Utilities|String|Append "  
 
 
 
 
 
 
 
 
 
 
 
 
                                     " "Teleport"))
        (bind _returnvalue (Actor|GetActorOfClass "/Game/VRTemplate/Blueprints/VRPawn.VRPawn_C"))
        (Default|KeyTeleport _returnvalue)
        (if (Variables|Default|GetKeyOpen)
          (Variables|Default|SetKeyOpen false)
          (Components|MoveComponentTo _key_2 (.location (Transformation|GetRelativeTransform _key_2)) (Variables|Default|GetClosedRotator) false false 0.2 true))
        (else
          (Variables|Default|SetKeyOpen true)
          (Components|MoveComponentTo _key (.location (Transformation|GetRelativeTransform _key)) (Variables|Default|GetOpenRotator) false false 0.2 true))))))

(fn ConstructionScript)