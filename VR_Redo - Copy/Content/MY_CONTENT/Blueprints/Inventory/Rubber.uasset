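; Rubber is an eraser inventory item that erases drawings on actors it touches.
; Holding the X or A button sets an Erase flag, which clears on release or when the item is not selected in its InventoryComponent.
; While selected and erasing, every Tick queries the Box for overlapping actors and calls Erase on any DrawComponent they have.
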(event EventBeginPlay)

(event Collision|EventActorBeginOverlap
  (params (OtherActor :type Actor%20Object%20Reference)))

(event EventTick
  (params (DeltaSeconds :type Float%20%28single-precision%29))
  (if (Variables|/Game/MY_CONTENT/Blueprints/Inventory/InventoryComponent.InventoryComponent_C|GetIsSelected (Variables|Default|GetInventoryComponent))
    (if (and (Variables|/Game/MY_CONTENT/Blueprints/Inventory/InventoryComponent.InventoryComponent_C|GetIsSelected (Variables|Default|GetInventoryComponent)) (Variables|Default|GetErase))
      (for _array_element (Collision|GetOverlappingActors (Variables|Default|GetBox) 0 :!class /Script/Engine.PrimitiveComponent)
        (Utilities|IsValid (Actor|GetComponentbyClass _array_element "/Game/MY_CONTENT/DrawComponents/DrawComponent.DrawComponent_C")
          (:Is%20Valid
            (Default|Erase (Actor|GetComponentbyClass _array_element "/Game/MY_CONTENT/DrawComponents/DrawComponent.DrawComponent_C"))))))
    (else
      (Variables|Default|SetErase false))))

(event EventButtonX
  (Variables|Default|SetErase true))

(event EventButtonA
  (Variables|Default|SetErase true))

(event EventARelease
  (Variables|Default|SetErase false))

(event EventXRelease
  (Variables|Default|SetErase false))

(fn ConstructionScript)