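; VR four-colour pen inventory item that draws on any actor with a DrawComponent.
; Controller buttons cycle the selection: the notch animates, the pen rotates 90 degrees per colour offset by the HandSwitcher hand, and the VRPawn reattaches it.
; SetColour then swaps the nib material and CurrentBrush, using dynamic brush materials created at BeginPlay.
; While selected, nib overlap finds the DrawComponent and Tick passes it the pen's transform.
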(event OnComponentBeginOverlap(NibCollision)
  (params (OverlappedComponent :type Primitive%20Component%20Object%20Reference) (OtherActor :type Actor%20Object%20Reference) (OtherComp :type Primitive%20Component%20Object%20Reference) (OtherBodyIndex :type Integer) (bFromSweep :type Boolean) (SweepResult :type Hit%20Result%20Structure%20%28by%20ref%29))
  (bind _returnvalue (Actor|GetComponentbyClass OtherActor "/Game/MY_CONTENT/DrawComponents/DrawComponent.DrawComponent_C"))
  (if (Variables|/Game/MY_CONTENT/Blueprints/Inventory/InventoryComponent.InventoryComponent_C|GetIsSelected (Variables|Components|GetInventoryComponent))
    (Utilities|IsValid _returnvalue
      (:Is%20Valid
        (Variables|Components|SetDrawComponent _returnvalue)
        (Variables|Default|SetDrawing true)))))

(event OnComponentEndOverlap(NibCollision)
  (params (OverlappedComponent :type Primitive%20Component%20Object%20Reference) (OtherActor :type Actor%20Object%20Reference) (OtherComp :type Primitive%20Component%20Object%20Reference) (OtherBodyIndex :type Integer))
  (if (Variables|/Game/MY_CONTENT/Blueprints/Inventory/InventoryComponent.InventoryComponent_C|GetIsSelected (Variables|Components|GetInventoryComponent))
    (Utilities|IsValid (Actor|GetComponentbyClass OtherActor "/Game/MY_CONTENT/DrawComponents/DrawComponent.DrawComponent_C")
      (:Is%20Valid
        (Variables|Default|SetDrawing false)
        (Variables|Components|SetDrawComponent 0)))))

(event EventTick
  (params (DeltaSeconds :type Float%20%28single-precision%29))
  (if (Variables|Default|GetDrawing)
    (Default|Draw (Variables|Components|GetDrawComponent) (Transformation|GetActorTransform self))))

(event EventButtonA
  ;[1 1 1] Return animation of current pin
  (Utilities|AnimUp
    (:Out
      ;[1 1 1] Increment/Decrement Pen selection
      (if (<= (Variables|Default|GetPenSelection) 0)
        (Variables|Default|SetPenSelection 3)
        (else
          (bind _result (Math|Integer|DecrementInt (stale _output_get))
            (:%20%20
              (bind _output_get (Variables|Default|SetPenSelection _result))))))
      (bind _returnvalue (Actor|GetActorOfClass "/Game/MY_CONTENT/Blueprints/Menu/HandSwitcher.HandSwitcher_C"))
      ;[1 1 1] Rotate Pen
      (if (Variables|/Game/MY_CONTENT/Blueprints/Menu/HandSwitcher.HandSwitcher_C|GetIsLeft _returnvalue)
        (Transformation|SetRelativeRotation (Variables|Components|GetInventoryComponent) (Math|Rotator|MakeRotator 33.0 25.0 (* (Variables|Default|GetPenSelection) 9e+01)) false false)
        (else
          (Transformation|SetRelativeRotation (Variables|Components|GetInventoryComponent) (Math|Rotator|MakeRotator 33.0 25.0 (+ (* (Variables|Default|GetPenSelection) 9e+01) 1.8e+02)) false false)))
      (bind _returnvalue_2 (Actor|GetActorOfClass "/Game/VRTemplate/Blueprints/VRPawn.VRPawn_C"))
      (Default|PenRe-Attach _returnvalue_2)
      ;[1 1 1] Animate next pin
      (Utilities|FlowControl|Delay 0.1)
      (Utilities|AnimDown
        (:Out
          ;[1 1 1] Set Pen Colour
          (Utilities|SetColour))))))

(event EventButtonB
  ;[1 1 1] Return animation of current pin
  (Utilities|AnimUp
    (:Out
      ;[1 1 1] Increment/Decrement Pen selection
      (if (>= (Variables|Default|GetPenSelection) 3)
        (Variables|Default|SetPenSelection 0)
        (else
          (bind _result (Math|Integer|IncrementInt (stale _output_get))
            (:%20%20
              (bind _output_get (Variables|Default|SetPenSelection _result))))))
      (bind _returnvalue (Actor|GetActorOfClass "/Game/MY_CONTENT/Blueprints/Menu/HandSwitcher.HandSwitcher_C"))
      ;[1 1 1] Rotate Pen
      (if (Variables|/Game/MY_CONTENT/Blueprints/Menu/HandSwitcher.HandSwitcher_C|GetIsLeft _returnvalue)
        (Transformation|SetRelativeRotation (Variables|Components|GetInventoryComponent) (Math|Rotator|MakeRotator 33.0 25.0 (* (Variables|Default|GetPenSelection) 9e+01)) false false)
        (else
          (Transformation|SetRelativeRotation (Variables|Components|GetInventoryComponent) (Math|Rotator|MakeRotator 33.0 25.0 (+ (* (Variables|Default|GetPenSelection) 9e+01) 1.8e+02)) false false)))
      (bind _returnvalue_2 (Actor|GetActorOfClass "/Game/VRTemplate/Blueprints/VRPawn.VRPawn_C"))
      (Default|PenRe-Attach _returnvalue_2)
      ;[1 1 1] Animate next pin
      (Utilities|FlowControl|Delay 0.1)
      (Utilities|AnimDown
        (:Out
          ;[1 1 1] Set Pen Colour
          (Utilities|SetColour))))))

(event EventButtonX
  ;[1 1 1] Return animation of current pin
  (Utilities|AnimUp
    (:Out
      ;[1 1 1] Increment/Decrement Pen selection
      (if (<= (Variables|Default|GetPenSelection) 0)
        (Variables|Default|SetPenSelection 3)
        (else
          (bind _result (Math|Integer|DecrementInt (stale _output_get))
            (:%20%20
              (bind _output_get (Variables|Default|SetPenSelection _result))))))
      (bind _returnvalue (Actor|GetActorOfClass "/Game/MY_CONTENT/Blueprints/Menu/HandSwitcher.HandSwitcher_C"))
      ;[1 1 1] Rotate Pen
      (if (Variables|/Game/MY_CONTENT/Blueprints/Menu/HandSwitcher.HandSwitcher_C|GetIsLeft _returnvalue)
        (Transformation|SetRelativeRotation (Variables|Components|GetInventoryComponent) (Math|Rotator|MakeRotator 33.0 25.0 (* (Variables|Default|GetPenSelection) 9e+01)) false false)
        (else
          (Transformation|SetRelativeRotation (Variables|Components|GetInventoryComponent) (Math|Rotator|MakeRotator 33.0 25.0 (+ (* (Variables|Default|GetPenSelection) 9e+01) 1.8e+02)) false false)))
      (bind _returnvalue_2 (Actor|GetActorOfClass "/Game/VRTemplate/Blueprints/VRPawn.VRPawn_C"))
      (Default|PenRe-Attach _returnvalue_2)
      ;[1 1 1] Animate next pin
      (Utilities|FlowControl|Delay 0.1)
      (Utilities|AnimDown
        (:Out
          ;[1 1 1] Set Pen Colour
          (Utilities|SetColour))))))

(event EventButtonY
  ;[1 1 1] Return animation of current pin
  (Utilities|AnimUp
    (:Out
      ;[1 1 1] Increment/Decrement Pen selection
      (if (>= (Variables|Default|GetPenSelection) 3)
        (Variables|Default|SetPenSelection 0)
        (else
          (bind _result (Math|Integer|IncrementInt (stale _output_get))
            (:%20%20
              (bind _output_get (Variables|Default|SetPenSelection _result))))))
      (bind _returnvalue (Actor|GetActorOfClass "/Game/MY_CONTENT/Blueprints/Menu/HandSwitcher.HandSwitcher_C"))
      ;[1 1 1] Rotate Pen
      (if (Variables|/Game/MY_CONTENT/Blueprints/Menu/HandSwitcher.HandSwitcher_C|GetIsLeft _returnvalue)
        (Transformation|SetRelativeRotation (Variables|Components|GetInventoryComponent) (Math|Rotator|MakeRotator 33.0 25.0 (* (Variables|Default|GetPenSelection) 9e+01)) false false)
        (else
          (Transformation|SetRelativeRotation (Variables|Components|GetInventoryComponent) (Math|Rotator|MakeRotator 33.0 25.0 (+ (* (Variables|Default|GetPenSelection) 9e+01) 1.8e+02)) false false)))
      (bind _returnvalue_2 (Actor|GetActorOfClass "/Game/VRTemplate/Blueprints/VRPawn.VRPawn_C"))
      (Default|PenRe-Attach _returnvalue_2)
      ;[1 1 1] Animate next pin
      (Utilities|FlowControl|Delay 0.1)
      (Utilities|AnimDown
        (:Out
          ;[1 1 1] Set Pen Colour
          (Utilities|SetColour))))))

(event EventBeginPlay
  (bind _returnvalue (Rendering|Material|CreateDynamicMaterialInstance "/Game/MY_CONTENT/DrawComponents/Brushes/RedBrush_MAT.RedBrush_MAT" "None" "None" :!class /Script/Engine.KismetMaterialLibrary))
  (Variables|Default|SetRed_Brush _returnvalue)
  (bind _returnvalue_2 (Rendering|Material|CreateDynamicMaterialInstance "/Game/MY_CONTENT/DrawComponents/Brushes/BlackBrush_MAT.BlackBrush_MAT" "None" "None" :!class /Script/Engine.KismetMaterialLibrary))
  (bind _output_get (Variables|Default|SetBlack_Brush _returnvalue_2))
  (bind _returnvalue_3 (Rendering|Material|CreateDynamicMaterialInstance "/Game/MY_CONTENT/DrawComponents/Brushes/GreenBrush_MAT.GreenBrush_MAT" "None" "None" :!class /Script/Engine.KismetMaterialLibrary))
  (Variables|Default|SetGreen_Brush _returnvalue_3)
  (bind _returnvalue_4 (Rendering|Material|CreateDynamicMaterialInstance "/Game/MY_CONTENT/DrawComponents/Brushes/BlueBrush_MAT.BlueBrush_MAT" "None" "None" :!class /Script/Engine.KismetMaterialLibrary))
  (Variables|Default|SetBlue_Brush _returnvalue_4)
  (Variables|Default|SetCurrent_Brush _output_get))

(fn ConstructionScript)

(fn SetPositioning
  (params (Left :type Boolean))
  (bind _rotation (Variables|Default|GetRotation))
  (if Left
    (Transformation|SetRelativeRotation (Variables|Components|GetInventoryComponent) (Variables|Default|GetRotation) false false)
    (else
      (Transformation|SetRelativeRotation (Variables|Components|GetInventoryComponent) (Math|Rotator|MakeRotator (.roll _rotation) (.pitch _rotation) 1.8e+02) false false))))