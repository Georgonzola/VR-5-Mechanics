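; A test actor that converts the VR pawn's left motion controller grip pose from world space into the actor's local space.
; Each tick it reads the grip position and rotation, makes a transform relative to the actor's transform, and prints the resulting location.
; It moves its Sphere component to that local X and Y at a fixed height, so the sphere follows the hand across a horizontal plane.
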(event EventBeginPlay)

(event Collision|EventActorBeginOverlap
  (params (OtherActor :type Actor%20Object%20Reference)))

(event EventTick
  (params (DeltaSeconds :type Float%20%28single-precision%29))
  (bind _returnvalue (Actor|GetActorOfClass "/Game/VRTemplate/Blueprints/VRPawn.VRPawn_C"))
  (bind _motioncontrollerdata (Class|HeadMountedDisplayFunctionLibrary|GetMotionControllerData (Variables|/Game/VRTemplate/Blueprints/VRPawn.VRPawn_C|GetMotionControllerLeft _returnvalue) "Left"))
  (Development|PrintString (Utilities|String|Append " 
 
 
 
 
 
 
 
 
 
 
 
 
 
 
 
 
 
                              " (Utilities|String|ToString(Vector) (.location (Math|Transform|MakeRelativeTransform (Math|Transform|MakeTransform (.gripposition _motioncontrollerdata) (Class|KismetMathLibrary|QuatRotator (.griprotation _motioncontrollerdata))) (Transformation|GetActorTransform self))))))
  (Components|MoveComponentTo (Variables|Default|GetSphere) (Math|Vector|MakeVector (.X (Math|Vector|BreakVector (.location (Math|Transform|MakeRelativeTransform (Math|Transform|MakeTransform (.gripposition _motioncontrollerdata) (Class|KismetMathLibrary|QuatRotator (.griprotation _motioncontrollerdata))) (Transformation|GetActorTransform self))))) (.Y (Math|Vector|BreakVector (.location (Math|Transform|MakeRelativeTransform (Math|Transform|MakeTransform (.gripposition _motioncontrollerdata) (Class|KismetMathLibrary|QuatRotator (.griprotation _motioncontrollerdata))) (Transformation|GetActorTransform self))))) 35.0) "0, 0, 0" false false 0.2 false))

(fn ConstructionScript)